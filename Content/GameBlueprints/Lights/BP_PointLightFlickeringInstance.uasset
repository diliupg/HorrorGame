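; Point light Blueprint that flickers endlessly during play between its normal intensity and a minimum flicker intensity.
; From BeginPlay, a self-looping retriggerable delay waits a random time between MinTIme and MaxTime, then a FlipFlop alternately applies the low and normal intensity to the light component.
; The construction script applies the normal intensity up front.
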(event `self.ReceiveBeginPlay`
  (bind _pointlightcomponent (`self.PointLightComponent`))
  (`KismetSystemLibrary.RetriggerableDelay` (`KismetMathLibrary.RandomFloatInRange` (`self.MinTIme`) (`self.MaxTime`)) :!label _label)
  (`/Engine/EditorBlueprintResources/StandardMacros.FlipFlop`
    (:`A`
      (`LightComponent.SetIntensity` _pointlightcomponent (`self.MinFlickerIntensity`))
      (goto _label))
    (:`B`
      (`LightComponent.SetIntensity` _pointlightcomponent (`self.Intensity`))
      (goto _label))))

(fn `UserConstructionScript`
  (`LightComponent.SetIntensity` (`self.PointLightComponent`) (`self.Intensity`)))